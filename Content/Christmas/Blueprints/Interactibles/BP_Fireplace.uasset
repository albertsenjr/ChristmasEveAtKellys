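; BP_Fireplace is an interactible fireplace for the Christmas game, with a part the player rotates through stick rotations.
; Beginning an interaction disables the player's character movement, and this Blueprint never re-enables it.
; Every Tick, whether interacting or not, it maps the player's StickRotations to a clamped quarter-turn roll on Cube1.
; Tick also prints Cube1's world pitch as debug output, although the driven axis is roll.
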(event EventBeginPlay
  (|CallParentFunction) ; This node is disabled and will not be called.\nDrag off pins to build functionality.
)

(event Collision|EventActorBeginOverlap
  (params (OtherActor :type Actor%20Object%20Reference))
  (|CallParentFunction OtherActor) ; This node is disabled and will not be called.\nDrag off pins to build functionality.
)

(event EventTick
  (params (DeltaSeconds :type Float%20%28single-precision%29))
  (bind _cube1 (Variables|Default|GetCube1))
  (|CallParentFunction DeltaSeconds)
  (Transformation|SetRelativeRotation _cube1 (Math|Rotator|MakeRotator (Math|Float|Clamp(Float) (* (Variables|/Game/ThirdPerson/Blueprints/BP_ThirdPersonCharacter.BP_ThirdPersonCharacter_C|GetStick%20rotations (Variables|Default|GetPlayer_REF)) -1.8e+02) -9e+01 0.0) 0.0 0.0) false false)
  (Development|PrintString (Utilities|String|ToString(Float) (.pitch (Transformation|GetWorldRotation _cube1)))))

(event EventBeginInteraction
  (Pawn|Components|CharacterMovement|DisableMovement (Variables|/Script/Engine.Character|GetCharacterMovement (Variables|Default|GetPlayer_REF))))

(fn ConstructionScript
  (|CallParentFunction))