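; BP_Statue is an interactable statue that temporarily takes over the player's view when interaction begins.
; BeginInteraction blends the view to the owner of its Camera over a few seconds, shows the cursor and switches to UI-only input.
; After a fixed delay, it cuts back to the owner of the player's FollowCamera, hides the cursor and restores game-only input.
; The player controller is cached at BeginPlay, and the return is purely timed.
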(event Input|EnhancedActionEvents|EnhancedInputActionIA_Return
  (params (ActionValue :type Boolean) (ElapsedSeconds :type Float%20%28double-precision%29) (TriggeredSeconds :type Float%20%28double-precision%29) (InputAction :type Input%20Action%20Object%20Reference :default "/Game/ThirdPerson/Input/Actions/IA_Return.IA_Return")))

(event EventBeginPlay
  (|CallParentFunction)
  (Variables|Default|SetPlayerController_REF (Game|GetPlayerController 0)))

(event Collision|EventActorBeginOverlap
  (params (OtherActor :type Actor%20Object%20Reference))
  (|CallParentFunction OtherActor) ; This node is disabled and will not be called.\nDrag off pins to build functionality.
)

(event EventTick
  (params (DeltaSeconds :type Float%20%28single-precision%29))
  (|CallParentFunction DeltaSeconds) ; This node is disabled and will not be called.\nDrag off pins to build functionality.
)

(event EventBeginInteraction
  (bind _playercontroller_ref (Variables|Default|GetPlayerController_REF))
  (bind _playercontroller_ref_2 (Variables|Default|GetPlayerController_REF))
  (Game|Player|SetViewTargetwithBlend _playercontroller_ref (Components|GetOwner (Variables|Default|GetCamera)) 3.0 "VTBlend_Linear" 0.0 false)
  (Variables|/Script/Engine.PlayerController|SetbShowMouseCursor _playercontroller_ref true)
  (Input|SetInputModeUIOnly (Variables|Default|GetPlayerController_REF) 0 "DoNotLock" false)
  (Utilities|FlowControl|Delay 5.0)
  (Game|Player|SetViewTargetwithBlend (Variables|Default|GetPlayerController_REF) (Components|GetOwner (Variables|/Game/ThirdPerson/Blueprints/BP_ThirdPersonCharacter.BP_ThirdPersonCharacter_C|GetFollowCamera (Variables|Default|GetPlayer_REF))) 0.0 "VTBlend_Linear" 0.0 false)
  (Variables|/Script/Engine.PlayerController|SetbShowMouseCursor _playercontroller_ref_2 false)
  (Input|SetInputModeGameOnly _playercontroller_ref_2 false))

(fn ConstructionScript
  (|CallParentFunction))