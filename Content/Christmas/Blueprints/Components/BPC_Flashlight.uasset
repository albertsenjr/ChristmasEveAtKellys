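; BPC_Flashlight is a component that runs the third-person player's flashlight and its battery, driving the SpotLight and state flags on the character.
; Toggleflashlight sets normal or UV color, switches the light and starts or clears a looping DepleteBatteryLife timer.
; Each tick of that timer drains clamped battery life, ten times faster in UV mode, and hides the light at minimum charge.
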(event EventBeginPlay
  (bind _asbp_third_person_character (Utilities|Casting|CastToBP_ThirdPersonCharacter (Game|GetPlayerCharacter 0)))
  (bind _output_get (Variables|Default|SetPlayer_REF _asbp_third_person_character)))

(event EventTick
  (params (DeltaSeconds :type Float%20%28single-precision%29)))

(fn DepleteBatteryLife
  (if (Variables|/Game/ThirdPerson/Blueprints/BP_ThirdPersonCharacter.BP_ThirdPersonCharacter_C|GetUVMode (Variables|Default|GetPlayer_REF))
    (Variables|Default|SetUVDepletionMultiplier 1e+01)
    (else
      (Variables|Default|SetUVDepletionMultiplier 1.0)))
  (Variables|Default|SetCurrentBatteryLife (Math|Float|Clamp(Float) (- (Variables|Default|GetCurrentBatteryLife) (* (Variables|Default|GetDepletionAmount) (Variables|Default|GetUVDepletionMultiplier))) (Variables|Default|GetMinBatteryLife) (Variables|Default|GetMaxBatteryLife)))
  (if (== (Variables|Default|GetCurrentBatteryLife) (Variables|Default|GetMinBatteryLife))
    (Rendering|SetVisibility (Variables|/Game/ThirdPerson/Blueprints/BP_ThirdPersonCharacter.BP_ThirdPersonCharacter_C|GetSpotLight (Variables|Default|GetPlayer_REF)) false false)))

(fn Toggleflashlight
  (bind _player_ref (Variables|Default|GetPlayer_REF))
  (bind _player_ref_2 (Variables|Default|GetPlayer_REF))
  (bind _player_ref_3 (Variables|Default|GetPlayer_REF))
  (bind _spotlight (Variables|/Game/ThirdPerson/Blueprints/BP_ThirdPersonCharacter.BP_ThirdPersonCharacter_C|GetSpotLight _player_ref_2))
  (Rendering|Components|Light|SetLightColor (Variables|/Game/ThirdPerson/Blueprints/BP_ThirdPersonCharacter.BP_ThirdPersonCharacter_C|GetSpotLight _player_ref_3) (select (Variables|/Game/ThirdPerson/Blueprints/BP_ThirdPersonCharacter.BP_ThirdPersonCharacter_C|GetUVMode _player_ref) (Variables|/Game/ThirdPerson/Blueprints/BP_ThirdPersonCharacter.BP_ThirdPersonCharacter_C|GetUVLightColor _player_ref) (Variables|/Game/ThirdPerson/Blueprints/BP_ThirdPersonCharacter.BP_ThirdPersonCharacter_C|GetLightColor _player_ref)) true)
  (if (Variables|/Game/ThirdPerson/Blueprints/BP_ThirdPersonCharacter.BP_ThirdPersonCharacter_C|GetIsFlashlightOn _player_ref_3)
    (if (> (Variables|Default|GetCurrentBatteryLife) (Variables|Default|GetMinBatteryLife))
      (Variables|/Game/ThirdPerson/Blueprints/BP_ThirdPersonCharacter.BP_ThirdPersonCharacter_C|SetIsFlashlightOn _player_ref_3 false)
      (Rendering|SetVisibility _spotlight false false)
      (Variables|/Game/ThirdPerson/Blueprints/BP_ThirdPersonCharacter.BP_ThirdPersonCharacter_C|SetUVMode (Variables|Default|GetPlayer_REF) false)
      (Utilities|Time|ClearTimerbyFunctionName 0 "DepleteBatteryLife"))
    (else
      (Variables|/Game/ThirdPerson/Blueprints/BP_ThirdPersonCharacter.BP_ThirdPersonCharacter_C|SetIsFlashlightOn _player_ref_3 true)
      (CallFunction|DepleteBatteryLife)
      (Rendering|SetVisibility _spotlight true false)
      (Utilities|Time|SetTimerbyFunctionName 0 "DepleteBatteryLife" (Variables|Default|GetDepletion%20speed) true))))

(fn Initialize
  (params (Player_REF :type BP%20Third%20Person%20Character%20Object%20Reference))
  (bind _output_get (Variables|Default|SetPlayer_REF Player_REF))
  (Variables|Default|SetFlashlight%20Light (Variables|/Game/ThirdPerson/Blueprints/BP_ThirdPersonCharacter.BP_ThirdPersonCharacter_C|GetSpotLight _output_get)))