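; Interactible slide puzzle actor that opens a 3x3 sliding puzzle UI when the player interacts with it.
; BeginPlay caches the player controller and creates the W_SlidePuzzle3x3 widget in a collapsed state.
; BeginInteraction blends the view to the owner of Camera, shows the mouse cursor, switches to UI-only input and displays the widget.
; This graph has no exit logic to restore the view or input.
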(event EventBeginPlay
  (|CallParentFunction)
  (Variables|Default|SetPlayerController_REF (Game|GetPlayerController 0))
  (bind _returnvalue (UserInterface|CreateWidget "/Game/Christmas/Widgets/W_SlidePuzzle3x3.W_SlidePuzzle3x3_C"))
  (bind _output_get (Variables|Default|SetSlidePuzzle_REF _returnvalue))
  (Widget|SetVisibility _output_get "Collapsed"))

(event Collision|EventActorBeginOverlap
  (params (OtherActor :type Actor%20Object%20Reference))
  (|CallParentFunction OtherActor) ; This node is disabled and will not be called.\nDrag off pins to build functionality.
)

(event EventTick
  (params (DeltaSeconds :type Float%20%28single-precision%29))
  (|CallParentFunction DeltaSeconds) ; This node is disabled and will not be called.\nDrag off pins to build functionality.
)

(event EventBeginInteraction
  (bind _playercontroller_ref (Variables|Default|GetPlayerController_REF))
  (Game|Player|SetViewTargetwithBlend _playercontroller_ref (Components|GetOwner (Variables|Default|GetCamera)) 3.0 "VTBlend_Linear" 0.0 false)
  (Variables|/Script/Engine.PlayerController|SetbShowMouseCursor _playercontroller_ref true)
  (Input|SetInputModeUIOnly (Variables|Default|GetPlayerController_REF) 0 "DoNotLock" false)
  (UserInterface|Viewport|AddtoViewport (Variables|Default|GetSlidePuzzle_REF) 0)
  (Widget|SetVisibility (Variables|Default|GetSlidePuzzle_REF) "Visible"))

(fn ConstructionScript
  (|CallParentFunction))