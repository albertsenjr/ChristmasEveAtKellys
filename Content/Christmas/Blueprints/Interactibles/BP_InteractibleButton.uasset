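; BP_InteractibleButton is an interactible button Blueprint that plays a simple press animation when interaction begins.
; On BeginInteraction, it snaps the ButtonTop component down along local Z, waits briefly with a Delay, then returns it to zero relative location.
; The graph holds only this visual feedback, with no Tick logic and no effect triggered on other objects.
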(event EventBeginPlay
  (|CallParentFunction) ; This node is disabled and will not be called.\nDrag off pins to build functionality.
)

(event Collision|EventActorBeginOverlap
  (params (OtherActor :type Actor%20Object%20Reference))
  (|CallParentFunction OtherActor) ; This node is disabled and will not be called.\nDrag off pins to build functionality.
)

(event EventTick
  (params (DeltaSeconds :type Float%20%28single-precision%29))
  (|CallParentFunction DeltaSeconds) ; This node is disabled and will not be called.\nDrag off pins to build functionality.
)

(event EventBeginInteraction
  (Transformation|SetRelativeLocation (Variables|Default|GetButtonTop) "0.000000,0.000000,-5.000000" false false)
  (Utilities|FlowControl|Delay 0.2)
  (Transformation|SetRelativeLocation (Variables|Default|GetButtonTop) "0.000000,0.000000,0.000000" false false))

(fn ConstructionScript
  (|CallParentFunction))