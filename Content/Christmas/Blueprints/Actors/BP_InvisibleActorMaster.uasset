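; Master actor for hidden objects revealed by the player's UV flashlight, swapping its cube and two planes between visible and invisible material instances.
; BeginPlay caches the third-person character and calls Reveal, which shows the meshes only when the flashlight, UV mode and UV-hit flag are all true.
; Tick only re-hides them as those conditions or capsule overlap lapse.
; Sphere-trace and Lightbox-overlap checks are left disconnected.
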(event OnComponentBeginOverlap(Box)
  (params (OverlappedComponent :type Primitive%20Component%20Object%20Reference) (OtherActor :type Actor%20Object%20Reference) (OtherComp :type Primitive%20Component%20Object%20Reference) (OtherBodyIndex :type Integer) (bFromSweep :type Boolean) (SweepResult :type Hit%20Result%20Structure%20%28by%20ref%29)))

(event OnComponentEndOverlap(Box)
  (params (OverlappedComponent :type Primitive%20Component%20Object%20Reference) (OtherActor :type Actor%20Object%20Reference) (OtherComp :type Primitive%20Component%20Object%20Reference) (OtherBodyIndex :type Integer)))

(event EventBeginPlay
  (bind _asbp_third_person_character (Utilities|Casting|CastToBP_ThirdPersonCharacter (Game|GetPlayerCharacter 0)))
  (Variables|Default|SetPlayer_REF _asbp_third_person_character)
  (CallFunction|Reveal))

(event Collision|EventActorBeginOverlap
  (params (OtherActor :type Actor%20Object%20Reference)))

(event EventTick
  (params (DeltaSeconds :type Float%20%28single-precision%29))
  (bind _player_ref (Variables|Default|GetPlayer_REF))
  (bind _player_ref_2 (Variables|Default|GetPlayer_REF))
  (if (and (not (Collision|IsOverlappingActor (Variables|/Game/ThirdPerson/Blueprints/BP_ThirdPersonCharacter.BP_ThirdPersonCharacter_C|GetCapsule _player_ref_2) (Variables|/Game/ThirdPerson/Blueprints/BP_ThirdPersonCharacter.BP_ThirdPersonCharacter_C|GetUVHit%20Actor _player_ref_2) :!class /Script/Engine.PrimitiveComponent)) (not (Variables|/Game/ThirdPerson/Blueprints/BP_ThirdPersonCharacter.BP_ThirdPersonCharacter_C|GetUVhittingTrue? _player_ref_2)))
    (CallFunction|HideMaterial :!label _label)
    (elif (not (and (Variables|/Game/ThirdPerson/Blueprints/BP_ThirdPersonCharacter.BP_ThirdPersonCharacter_C|GetIsFlashlightOn _player_ref) (Variables|/Game/ThirdPerson/Blueprints/BP_ThirdPersonCharacter.BP_ThirdPersonCharacter_C|GetUVMode _player_ref)))
      (goto _label))))

(event EventReveal
  (bind _player_ref (Variables|Default|GetPlayer_REF))
  (bind _player_ref_2 (Variables|Default|GetPlayer_REF))
  (bind _uvhittingtrue_ (Variables|/Game/ThirdPerson/Blueprints/BP_ThirdPersonCharacter.BP_ThirdPersonCharacter_C|GetUVhittingTrue? _player_ref_2))
  (if (Math|Boolean|ANDBoolean (Variables|/Game/ThirdPerson/Blueprints/BP_ThirdPersonCharacter.BP_ThirdPersonCharacter_C|GetIsFlashlightOn _player_ref_2) (Variables|/Game/ThirdPerson/Blueprints/BP_ThirdPersonCharacter.BP_ThirdPersonCharacter_C|GetUVMode _player_ref_2) _uvhittingtrue_)
    (CallFunction|ShowMaterial)
    (else
      (CallFunction|HideMaterial)))
  (if (and (not (Collision|IsOverlappingActor (Variables|/Game/ThirdPerson/Blueprints/BP_ThirdPersonCharacter.BP_ThirdPersonCharacter_C|GetCapsule _player_ref_2) (Variables|/Game/ThirdPerson/Blueprints/BP_ThirdPersonCharacter.BP_ThirdPersonCharacter_C|GetUVHit%20Actor _player_ref_2) :!class /Script/Engine.PrimitiveComponent)) (not _uvhittingtrue_))
    (CallFunction|HideMaterial :!label _label)
    (elif (not (and (Variables|/Game/ThirdPerson/Blueprints/BP_ThirdPersonCharacter.BP_ThirdPersonCharacter_C|GetIsFlashlightOn _player_ref) (Variables|/Game/ThirdPerson/Blueprints/BP_ThirdPersonCharacter.BP_ThirdPersonCharacter_C|GetUVMode _player_ref)))
      (goto _label))))

(fn ConstructionScript)

(fn UVlight
  (bind _player_ref (Variables|Default|GetPlayer_REF))
  (bind _cube (Variables|Default|GetCube))
  (if (Math|Boolean|ANDBoolean (Variables|/Game/ThirdPerson/Blueprints/BP_ThirdPersonCharacter.BP_ThirdPersonCharacter_C|GetIsFlashlightOn _player_ref) (Variables|/Game/ThirdPerson/Blueprints/BP_ThirdPersonCharacter.BP_ThirdPersonCharacter_C|GetUVMode _player_ref) (Collision|IsOverlappingActor (Variables|/Game/ThirdPerson/Blueprints/BP_ThirdPersonCharacter.BP_ThirdPersonCharacter_C|GetCapsule _player_ref) self :!class /Script/Engine.PrimitiveComponent))
    (Rendering|Material|SetMaterial _cube 0 "/Game/Christmas/Blueprints/M_invis_Inst.M_invis_Inst")
    (else
      (Rendering|Material|SetMaterial _cube 0 "/Game/Christmas/Blueprints/M_invis_InstOff.M_invis_InstOff"))))

(fn ShowMaterial
  (Rendering|Material|SetMaterial (Variables|Default|GetCube) 0 "/Game/Christmas/Blueprints/M_invis_Inst.M_invis_Inst"))

(fn HideMaterial
  (Rendering|Material|SetMaterial (Variables|Default|GetCube) 0 "/Game/Christmas/Blueprints/M_invis_InstOff.M_invis_InstOff"))

(fn UVMaterial
  (bind _player_ref (Variables|Default|GetPlayer_REF))
  (if (Math|Boolean|ANDBoolean (Variables|/Game/ThirdPerson/Blueprints/BP_ThirdPersonCharacter.BP_ThirdPersonCharacter_C|GetIsFlashlightOn _player_ref) (Variables|/Game/ThirdPerson/Blueprints/BP_ThirdPersonCharacter.BP_ThirdPersonCharacter_C|GetUVMode _player_ref) (Variables|/Game/ThirdPerson/Blueprints/BP_ThirdPersonCharacter.BP_ThirdPersonCharacter_C|GetUVhittingTrue? _player_ref))
    (CallFunction|ShowMaterial)
    (else
      (CallFunction|HideMaterial))))