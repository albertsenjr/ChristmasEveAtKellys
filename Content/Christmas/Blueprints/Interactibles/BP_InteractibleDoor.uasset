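; Interactible door actor that swings when a player interacts with it, unless it is locked.
; BeginInteraction prints a debug message if Locked, otherwise flips the Open flag and snaps the Door to 90 degrees in one direction or the other.
; Leaving the Sphere trigger resets the rotation to zero without clearing Open.
; The Rotate_TL timeline and delayed reset are unconnected, so movement is instant.
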(event OnComponentEndOverlap(Sphere)
  (params (OverlappedComponent :type Primitive%20Component%20Object%20Reference) (OtherActor :type Actor%20Object%20Reference) (OtherComp :type Primitive%20Component%20Object%20Reference) (OtherBodyIndex :type Integer))
  (Transformation|SetRelativeRotation (Variables|Default|GetDoor) "0, 0, 0" false false))

(event EventBeginPlay
  (|CallParentFunction) ; This node is disabled and will not be called.\nDrag off pins to build functionality.
)

(event Collision|EventActorBeginOverlap
  (params (OtherActor :type Actor%20Object%20Reference))
  (|CallParentFunction OtherActor) ; This node is disabled and will not be called.\nDrag off pins to build functionality.
)

(event EventTick
  (params (DeltaSeconds :type Float%20%28single-precision%29))
  (|CallParentFunction DeltaSeconds) ; This node is disabled and will not be called.\nDrag off pins to build functionality.
)

(event EventBeginInteraction
  (bind _door (Variables|Default|GetDoor))
  (if (Variables|Default|GetLocked?)
    (Development|PrintString "This door is LOCKED")
    (elif (Variables|Default|GetOpen?)
      (Variables|Default|SetOpen? false)
      (Transformation|SetRelativeRotation _door "0.0,90.0,0.0" false false)
      (else
        (Variables|Default|SetOpen? true)
        (Transformation|SetRelativeRotation _door "0.000000,-90.000000,0.000000" false false)))))

(fn ConstructionScript
  (|CallParentFunction))