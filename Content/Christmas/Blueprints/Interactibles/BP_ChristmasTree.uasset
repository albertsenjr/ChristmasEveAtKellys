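; Interactable Christmas tree that lets the player decorate six ornaments with chosen materials through the W_DecorateTree widget.
; BeginInteraction blends the view to the tree's camera, shows the widget and switches to UI-only input.
; Tick polls the widget, applying its material to the selected ornament and resetting the selection to zero, which maps to Ornament6.
; The widget's exit flag or Exit event restores the player camera and game input.
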(event Custom|Exit
  (bind _playercontroller_ref (Variables|Default|GetPlayerController_REF))
  (Widget|SetVisibility (Variables|Default|GetW_DecorateTree_REF) "Collapsed")
  (Game|Player|SetViewTargetwithBlend (Variables|Default|GetPlayerController_REF) (Components|GetOwner (Variables|/Game/ThirdPerson/Blueprints/BP_ThirdPersonCharacter.BP_ThirdPersonCharacter_C|GetFollowCamera (Variables|Default|GetPlayer_REF))) 0.0 "VTBlend_Linear" 0.0 false)
  (Variables|/Script/Engine.PlayerController|SetbShowMouseCursor _playercontroller_ref false)
  (Input|SetInputModeGameOnly _playercontroller_ref false)
  (Variables|/Game/Christmas/Widgets/W_DecorateTree.W_DecorateTree_C|SetExit (Variables|Default|GetW_DecorateTree_REF) false))

(event EventBeginPlay
  (|CallParentFunction)
  (Variables|Default|SetPlayerController_REF (Game|GetPlayerController 0))
  (bind _returnvalue (UserInterface|CreateWidget "/Game/Christmas/Widgets/W_DecorateTree.W_DecorateTree_C"))
  (bind _output_get (Variables|Default|SetW_DecorateTree_REF _returnvalue))
  (Widget|SetVisibility _output_get "Collapsed"))

(event Collision|EventActorBeginOverlap
  (params (OtherActor :type Actor%20Object%20Reference))
  (|CallParentFunction OtherActor) ; This node is disabled and will not be called.\nDrag off pins to build functionality.
)

(event EventTick
  (params (DeltaSeconds :type Float%20%28single-precision%29))
  (bind _w_decoratetree_ref (Variables|Default|GetW_DecorateTree_REF))
  (bind _playercontroller_ref (Variables|Default|GetPlayerController_REF))
  (|CallParentFunction DeltaSeconds)
  (CallFunction|SetOrnamentColor)
  (if (Variables|/Game/Christmas/Widgets/W_DecorateTree.W_DecorateTree_C|GetExit _w_decoratetree_ref)
    (Widget|SetVisibility (Variables|Default|GetW_DecorateTree_REF) "Collapsed")
    (Game|Player|SetViewTargetwithBlend (Variables|Default|GetPlayerController_REF) (Components|GetOwner (Variables|/Game/ThirdPerson/Blueprints/BP_ThirdPersonCharacter.BP_ThirdPersonCharacter_C|GetFollowCamera (Variables|Default|GetPlayer_REF))) 0.0 "VTBlend_Linear" 0.0 false)
    (Variables|/Script/Engine.PlayerController|SetbShowMouseCursor _playercontroller_ref false)
    (Input|SetInputModeGameOnly _playercontroller_ref false)
    (Variables|/Game/Christmas/Widgets/W_DecorateTree.W_DecorateTree_C|SetExit _w_decoratetree_ref false)))

(event EventBeginInteraction
  (bind _playercontroller_ref (Variables|Default|GetPlayerController_REF))
  (Game|Player|SetViewTargetwithBlend _playercontroller_ref (Components|GetOwner (Variables|Default|GetCamera)) 3.0 "VTBlend_Linear" 0.0 false)
  (Variables|/Script/Engine.PlayerController|SetbShowMouseCursor _playercontroller_ref true)
  (Input|SetInputModeUIOnly (Variables|Default|GetPlayerController_REF) 0 "DoNotLock" false)
  (UserInterface|Viewport|AddtoViewport (Variables|Default|GetW_DecorateTree_REF) 0)
  (Widget|SetVisibility (Variables|Default|GetW_DecorateTree_REF) "Visible"))

(fn ConstructionScript
  (|CallParentFunction))

(fn SetOrnamentColor
  (bind _w_decoratetree_ref (Variables|Default|GetW_DecorateTree_REF))
  (Rendering|Material|SetMaterial (Utilities|Select :Index (Variables|/Game/Christmas/Widgets/W_DecorateTree.W_DecorateTree_C|GetSelectedOrnament _w_decoratetree_ref) :Option%200 (Variables|Default|GetOrnament6) :Option%201 (Variables|Default|GetOrnament1) :Option%202 (Variables|Default|GetOrnament2) :Option%203 (Variables|Default|GetOrnament3) :Option%204 (Variables|Default|GetOrnament4) :Option%205 (Variables|Default|GetOrnament5)) 0 (Variables|/Game/Christmas/Widgets/W_DecorateTree.W_DecorateTree_C|GetSelectedMaterial _w_decoratetree_ref))
  (Variables|/Game/Christmas/Widgets/W_DecorateTree.W_DecorateTree_C|SetSelectedOrnament _w_decoratetree_ref 0))